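; Bow equipment Blueprint that automatically holds the weapon's sub-action while an AI-controlled character has the bow equipped.
; After the parent EndEquip and Unequip logic runs, it checks that the owner's controller is an AIController.
; If so, it calls SubActionPressed on the owner's CWeaponComponent when equipping ends and SubActionReleased on unequip.
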(event EventEndEquip
  (bind _ownercharacter (Variables|Default|GetOwnerCharacter))
  (bind _returnvalue (Actor|GetComponentbyClass _ownercharacter "/Script/BODYCREDIT.CWeaponComponent"))
  (|CallParentFunction)
  (Utilities|Casting|CastToAIController (Pawn|GetController (Variables|Default|GetOwnerCharacter)))
  (Utilities|IsValid _returnvalue
    (:Is%20Valid
      (Class|CWeaponComponent|SubActionPressed _returnvalue))))

(event EventUnequip
  (bind _ownercharacter (Variables|Default|GetOwnerCharacter))
  (bind _returnvalue (Actor|GetComponentbyClass _ownercharacter "/Script/BODYCREDIT.CWeaponComponent"))
  (|CallParentFunction)
  (Utilities|Casting|CastToAIController (Pawn|GetController (Variables|Default|GetOwnerCharacter)))
  (Utilities|IsValid _returnvalue
    (:Is%20Valid
      (Class|CWeaponComponent|SubActionReleased _returnvalue))))